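; Scene 9 professor NPC that stages a scripted dialogue with the player's MotionControllerPawn_Darts.
; The construction script loads lines from DT_Conversation_Scene9.
; BeginPlay switches input to UI-only, turns the camera toward the professor (ignoring the target argument), then calls an empty Move and Talk.
; Each Talk call shows the next line in WBP_DialogueBox, triggers a player nod at one index, and restores game input after the last.
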(event Custom|Move)

(event Custom|Event%20TakeAction
  (CallFunction|Move)
  (Utilities|FlowControl|Delay 0.5)
  (CallFunction|Talk))

(event Custom|Player%20Nod
  (Variables|/Game/CrystalVision2/UI/WBP_DialogueBox.WBP_DialogueBox_C|SetCanClick (Variables|Default|GetUI) false)
  (Default|NodDown (Variables|Default|GetPlayer) 30)
  (Utilities|FlowControl|Delay 0.5)
  (Default|NodUp (Variables|Default|GetPlayer) 30)
  (Utilities|FlowControl|Delay 0.5)
  (Default|NodDown (Variables|Default|GetPlayer) 30)
  (Utilities|FlowControl|Delay 0.5)
  (Default|NodUp (Variables|Default|GetPlayer) 30))

(event EventBeginPlay
  (|CallParentFunction)
  (Utilities|FlowControl|Sequence
    (:then_1
      (bind _returnvalue (Actor|GetActorOfClass "/Game/Darts/Characters/VRPawn/MotionControllerPawn_Darts.MotionControllerPawn_Darts_C"))
      (Variables|Default|SetPlayer _returnvalue)
      (Utilities|FlowControl|Delay 1.0)
      (CallFunction|DisablePlayerInput)
      (Utilities|FlowControl|Delay 0.5)
      ;[1 1 1] Assign the location of the book
      (CallFunction|RotatePlayerCamerato "0, 0, 0")
      (Utilities|FlowControl|Delay 2.0)
      (CallFunction|EventTakeAction))))

(event Collision|EventActorBeginOverlap
  (params (OtherActor :type Actor%20Object%20Reference))
  (|CallParentFunction OtherActor) ; This node is disabled and will not be called.\nDrag off pins to build functionality.
)

(event EventTick
  (params (DeltaSeconds :type Float%20%28single-precision%29))
  (|CallParentFunction DeltaSeconds) ; This node is disabled and will not be called.\nDrag off pins to build functionality.
)

(event EventTalk
  (bind _returnvalue (Game|GetPlayerController 0))
  (if (< (Variables|Default|GetTextIDX) (Utilities|Array|Length (Variables|Default|GetTexts)))
    (if (== (Variables|Default|GetTextIDX) 4)
      (CallFunction|PlayerNod))
    (Utilities|IsValid (Variables|Default|GetUI)
      (:Is%20Valid
        _)
      (:Is%20Not%20Valid
        (bind _returnvalue_2 (UserInterface|CreateWidget "/Game/CrystalVision2/UI/WBP_DialogueBox.WBP_DialogueBox_C" _returnvalue))
        (bind _output_get (Variables|Default|SetUI _returnvalue_2))
        (UserInterface|Viewport|AddtoViewport _output_get 0)
        (Input|SetInputModeUIOnly _returnvalue (Variables|Default|GetUI) "DoNotLock" true)
        (Variables|/Game/CrystalVision2/UI/WBP_DialogueBox.WBP_DialogueBox_C|SetOwner (Variables|Default|GetUI) self)))
    (Rendering|Components|TextRender|SetText (Variables|/Game/CrystalVision2/UI/WBP_DialogueBox.WBP_DialogueBox_C|GetTalkText (Variables|Default|GetUI)) (Utilities|Array|Get(acopy) (Variables|Default|GetTexts) (Variables|Default|GetTextIDX)))
    (Math|Integer|IncrementInt (Variables|Default|GetTextIDX)
      (:%20%20
        (Variables|/Game/CrystalVision2/UI/WBP_DialogueBox.WBP_DialogueBox_C|SetCanClick (Variables|Default|GetUI) true)))
    (else
      (Widget|RemovefromParent (Variables|Default|GetUI))
      (Input|SetInputModeGameOnly (Game|GetPlayerController 0) true))))

(fn ConstructionScript
  (|CallParentFunction)
  (bind _outrownames (DataTable|GetDataTableRowNames "/Game/CrystalVision2/Structs/DT_Conversation_Scene9.DT_Conversation_Scene9"))
  (for _array_element _outrownames
    (bind _returnvalue (Utilities|GetDataTableRow "/Game/CrystalVision2/Structs/DT_Conversation_Scene9.DT_Conversation_Scene9" _array_element)
      (:then
        (Utilities|Array|Add (Variables|Default|GetTexts) (Utilities|Struct|BreakS_Dialogue _returnvalue))))))

(fn DisablePlayerInput
  (Utilities|IsValid (Variables|Default|GetPlayer)
    (:Is%20Valid
      (Input|SetInputModeUIOnly (Game|GetPlayerController 0) 0 "DoNotLock" true))))

(fn RotatePlayerCamerato
  (params (Target :type Vector))
  (Utilities|IsValid (Variables|Default|GetPlayer)
    (:Is%20Valid
      ;[1 1 1] Use function input when location is available
      (Default|RotateCameraatRate (Variables|Default|GetPlayer) (Transformation|GetActorLocation) 1.0))))