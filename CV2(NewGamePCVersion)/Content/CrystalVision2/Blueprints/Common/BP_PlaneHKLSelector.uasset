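; BP_PlaneHKLSelector is a shootable control that adjusts one HKL plane index for crystal visualization.
; BP_Bullet overlaps on its U and D components step the value up or down, clamped between -5 and 5.
; When the Displayer reference is valid, each step passes the index slot and value to its UpdateHKL and refreshes the selector's text render.
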(event OnComponentBeginOverlap(D)
  (params (OverlappedComponent :type Primitive%20Component%20Object%20Reference) (OtherActor :type Actor%20Object%20Reference) (OtherComp :type Primitive%20Component%20Object%20Reference) (OtherBodyIndex :type Integer) (bFromSweep :type Boolean) (SweepResult :type Hit%20Result%20Structure%20%28by%20ref%29))
  (Utilities|Casting|CastToBP_Bullet OtherActor)
  (CallFunction|Decrease))

(event OnComponentBeginOverlap(U)
  (params (OverlappedComponent :type Primitive%20Component%20Object%20Reference) (OtherActor :type Actor%20Object%20Reference) (OtherComp :type Primitive%20Component%20Object%20Reference) (OtherBodyIndex :type Integer) (bFromSweep :type Boolean) (SweepResult :type Hit%20Result%20Structure%20%28by%20ref%29))
  (Utilities|Casting|CastToBP_Bullet OtherActor)
  (CallFunction|Increase))

(event EventBeginPlay)

(event Collision|EventActorBeginOverlap
  (params (OtherActor :type Actor%20Object%20Reference)))

(event EventTick
  (params (DeltaSeconds :type Float%20%28single-precision%29)))

(fn ConstructionScript)

(fn Increase
  (bind _displayer (Variables|Default|GetDisplayer))
  (Variables|Default|Setvalue (Math|Integer|Min(Integer) (+ (Variables|Default|Getvalue) 1) 5))
  (Utilities|IsValid _displayer
    (:Is%20Valid
      (Default|UpdateHKL _displayer (Variables|Default|GetHKLidx) (Variables|Default|Getvalue))
      (CallFunction|RenderText))))

(fn Decrease
  (bind _displayer (Variables|Default|GetDisplayer))
  (Variables|Default|Setvalue (Math|Integer|Max(Integer) (- (Variables|Default|Getvalue) 1) -5))
  (Utilities|IsValid _displayer
    (:Is%20Valid
      (Default|UpdateHKL _displayer (Variables|Default|GetHKLidx) (Variables|Default|Getvalue))
      (CallFunction|RenderText))))

(fn RenderText
  (Rendering|Components|TextRender|SetText (Variables|Default|GetTextRender) (Utilities|Text|ToText(Integer) (Variables|Default|Getvalue))))