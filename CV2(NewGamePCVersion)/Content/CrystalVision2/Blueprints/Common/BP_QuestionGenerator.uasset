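; BP_QuestionGenerator sequences a quiz, presenting one set of question board, total score board and quiz module at a time.
; Shortly after BeginPlay, NextQuestion moves the current set from parallel arrays to stored transforms, calls Begin on the module and increments QuizID.
; Each later NextQuestion call first destroys the previous set.
; When the question boards run out, it spawns a Prof9 NPC spawner and destroys itself.
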(event Custom|NextQuestion
  (if (> (Variables|Default|GetQuizID) 0)
    (CallFunction|DestroyCurrent))
  (if (< (Variables|Default|GetQuizID) (Utilities|Array|Length (Variables|Default|GetQuestionBoards)))
    (Utilities|FlowControl|Sequence
      (:then_0
        (Transformation|SetActorLocationAndRotation (Utilities|Array|Get(acopy) (Variables|Default|GetQuestionBoards) (Variables|Default|GetQuizID)) (Variables|Default|GetQuestionBoardLocation) (Variables|Default|GetQuestionBoardRotation)))
      (:then_1
        (Transformation|SetActorLocationAndRotation (Utilities|Array|Get(acopy) (Variables|Default|GetTotalScoreBoards) (Variables|Default|GetQuizID)) (Variables|Default|GetTotalScoreBoardLocation) (Variables|Default|GetTotalScoreBoardRotation)))
      (:then_2
        (Transformation|SetActorLocationAndRotation (Utilities|Array|Get(acopy) (Variables|Default|GetQuizModules) (Variables|Default|GetQuizID)) (Variables|Default|GetQuizModuleLocation) (Variables|Default|GetQuizModuleRotation)))
      (:then_3
        (Default|Begin (Utilities|Array|Get(acopy) (Variables|Default|GetQuizModules) (Variables|Default|GetQuizID)))
        (Math|Integer|IncrementInt (Variables|Default|GetQuizID))))
    (else
      (Game|SpawnActorfromClass "/Game/CrystalVision2/Blueprints/Common/BP_NPC_Prof9_Spawner.BP_NPC_Prof9_Spawner_C" (Math|Transform|MakeTransform "-10.000000,-190.000000,50.000000" "0, 0, 0" "1.000000,1.000000,1.000000") "Undefined" "MultiplyWithRoot" 0 0)
      (Actor|DestroyActor))))

(event EventBeginPlay
  (Utilities|FlowControl|Delay 0.5)
  (CallFunction|NextQuestion))

(event Collision|EventActorBeginOverlap
  (params (OtherActor :type Actor%20Object%20Reference)))

(event EventTick
  (params (DeltaSeconds :type Float%20%28single-precision%29)))

(fn ConstructionScript)

(fn DestroyCurrent
  (Utilities|FlowControl|Sequence
    (:then_0
      (Actor|DestroyActor (Utilities|Array|Get(acopy) (Variables|Default|GetQuestionBoards) (- (Variables|Default|GetQuizID) 1))))
    (:then_1
      (Actor|DestroyActor (Utilities|Array|Get(acopy) (Variables|Default|GetTotalScoreBoards) (- (Variables|Default|GetQuizID) 1))))
    (:then_2
      (Actor|DestroyActor (Utilities|Array|Get(acopy) (Variables|Default|GetQuizModules) (- (Variables|Default|GetQuizID) 1))))))