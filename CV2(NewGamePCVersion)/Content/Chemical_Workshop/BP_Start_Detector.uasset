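; BP_Start_Detector is a one-shot trigger in the Chemical Workshop that brings in the professor NPC when the player's MotionControllerPawn_Darts enters its collision box.
; It spawns BP_NPC_Professor at a stored location and rotation, then looks up the first Darts pawn in the world.
; If that pawn is valid, it rotates its camera to a fixed rotation and starts the professor talking.
; The detector destroys itself either way.
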(event OnComponentBeginOverlap(CollisionBox)
  (params (OverlappedComponent :type Primitive%20Component%20Object%20Reference) (OtherActor :type Actor%20Object%20Reference) (OtherComp :type Primitive%20Component%20Object%20Reference) (OtherBodyIndex :type Integer) (bFromSweep :type Boolean) (SweepResult :type Hit%20Result%20Structure%20%28by%20ref%29))
  (Utilities|Casting|CastToMotionControllerPawn_Darts OtherActor)
  (bind _returnvalue (Game|SpawnActorfromClass "/Game/CrystalVision2/Blueprints/Common/BP_NPC_Professor.BP_NPC_Professor_C" (Math|Transform|MakeTransform (Variables|Default|GetSpawnLocation) (Variables|Default|GetSpawnRotation) "1.000000,1.000000,1.000000") "Undefined" "MultiplyWithRoot" 0 0))
  (bind _outactors (Actor|GetAllActorsOfClass "/Game/Darts/Characters/VRPawn/MotionControllerPawn_Darts.MotionControllerPawn_Darts_C"))
  (Utilities|IsValid (Utilities|Array|Get(acopy) _outactors)
    (:Is%20Valid
      (Default|RotateCamera (Utilities|Array|Get(acopy) _outactors) "-10.000000,105.000000,0.000000")
      (Default|Talk _returnvalue)
      (Actor|DestroyActor))
    (:Is%20Not%20Valid
      (Actor|DestroyActor))))

(event EventBeginPlay
  (|CallParentFunction) ; This node is disabled and will not be called.\nDrag off pins to build functionality.
)

(event Collision|EventActorBeginOverlap
  (params (OtherActor :type Actor%20Object%20Reference))
  (|CallParentFunction OtherActor) ; This node is disabled and will not be called.\nDrag off pins to build functionality.
)

(event EventTick
  (params (DeltaSeconds :type Float%20%28single-precision%29))
  (|CallParentFunction DeltaSeconds) ; This node is disabled and will not be called.\nDrag off pins to build functionality.
)

(fn ConstructionScript
  (|CallParentFunction))