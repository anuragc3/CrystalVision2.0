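; Professor NPC for Scene 23 that delivers a scripted conversation, then starts moving and hands off to the showcase map.
; The construction script loads sentences and path destinations from two DataTables.
; Each Talk call shows the next line in a UI-only dialogue widget, then restores game input and calls Move.
; Move recursively issues AI moves from both immediate and success pins, then fades out and opens the level.
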(event Custom|Move
  (if (< (Variables|Default|GetMoveDestIDX) (Utilities|Array|Length (Variables|Default|GetMoveDest)))
    ;[1 1 1] Make sure you have Nav Mesh placed in the level
    (AI|AIMoveTo self (Utilities|Array|Get(acopy) (Variables|Default|GetMoveDest) (Variables|Default|GetMoveDestIDX)) 0 0.1 false
      (:then
        _)
      (:OnSuccess
        _))
    (Math|Integer|IncrementInt (Variables|Default|GetMoveDestIDX)
      (:%20%20
        (CallFunction|Move)))
    (elif (== (Variables|Default|GetMoveDestIDX) (Utilities|Array|Length (Variables|Default|GetMoveDest)))
      ;[1 1 1] Link these 2 parts to fade out the camera and AFTER delta seconds, tp the player to a new level
      (CameraFades|StartCameraFade :self (Game|GetPlayerCameraManager 0) :ToAlpha 1.0 :Duration 2.0 :bShouldFadeAudio true :bHoldWhenFinished true)
      (Utilities|FlowControl|Delay 3.0)
      (Game|OpenLevel(byObjectReference) "/Game/Crystal_cave/Maps/L_showcase_map.L_showcase_map"))))

(event EventBeginPlay
  (|CallParentFunction) ; This node is disabled and will not be called.\nDrag off pins to build functionality.
)

(event Collision|EventActorBeginOverlap
  (params (OtherActor :type Actor%20Object%20Reference))
  (|CallParentFunction OtherActor) ; This node is disabled and will not be called.\nDrag off pins to build functionality.
)

(event EventTick
  (params (DeltaSeconds :type Float%20%28single-precision%29))
  (|CallParentFunction DeltaSeconds) ; This node is disabled and will not be called.\nDrag off pins to build functionality.
)

(event EventTalk
  (bind _returnvalue (Game|GetPlayerController 0))
  (if (< (Variables|Default|GetTextIDX) (Utilities|Array|Length (Variables|Default|GetTexts)))
    (Utilities|IsValid (Variables|Default|GetUI)
      (:Is%20Valid
        _)
      (:Is%20Not%20Valid
        (bind _returnvalue_2 (UserInterface|CreateWidget "/Game/CrystalVision2/UI/WBP_DialogueBox.WBP_DialogueBox_C" _returnvalue))
        (bind _output_get (Variables|Default|SetUI _returnvalue_2))
        (UserInterface|Viewport|AddtoViewport _output_get 0)
        (Input|SetInputModeUIOnly _returnvalue (Variables|Default|GetUI) "DoNotLock" true)
        (Variables|/Game/CrystalVision2/UI/WBP_DialogueBox.WBP_DialogueBox_C|SetOwner (Variables|Default|GetUI) self)))
    (Rendering|Components|TextRender|SetText (Variables|/Game/CrystalVision2/UI/WBP_DialogueBox.WBP_DialogueBox_C|GetTalkText (Variables|Default|GetUI)) (Utilities|Array|Get(acopy) (Variables|Default|GetTexts) (Variables|Default|GetTextIDX)))
    (Math|Integer|IncrementInt (Variables|Default|GetTextIDX))
    (else
      (Widget|RemovefromParent (Variables|Default|GetUI))
      (Input|SetInputModeGameOnly (Game|GetPlayerController 0) true)
      (CallFunction|Move))))

(fn ConstructionScript
  (|CallParentFunction)
  (Utilities|FlowControl|Sequence
    (:then_0
      (bind _outrownames (DataTable|GetDataTableRowNames "/Game/CrystalVision2/Structs/DT_Conversation_Scene23.DT_Conversation_Scene23"))
      (for _array_element _outrownames
        (bind _returnvalue (Utilities|GetDataTableRow "/Game/CrystalVision2/Structs/DT_Conversation_Scene23.DT_Conversation_Scene23" _array_element)
          (:then
            (Utilities|Array|Add (Variables|Default|GetTexts) (Utilities|Struct|BreakS_Dialogue _returnvalue))))))
    (:then_1
      ;[1 1 1] @TODO: link this part to Sequence 1 when dests has been specified (update those dest in ./CrystalVision2.0/Struct/DT_Prof_Path)
      (bind _outrownames_2 (DataTable|GetDataTableRowNames "/Game/CrystalVision2/Structs/DT_Prof_Path.DT_Prof_Path"))
      (for _array_element_2 _outrownames_2
        (bind _returnvalue_2 (Utilities|GetDataTableRow "/Game/CrystalVision2/Structs/DT_Prof_Path.DT_Prof_Path" _array_element_2)
          (:then
            (Utilities|Array|Add (Variables|Default|GetMoveDest) (Utilities|Struct|BreakS_AI_Dest _returnvalue_2))))))))