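; Test actor that feeds an oriented cube's frame to a dynamic material on its Plane component.
; The construction script creates the material instance; Tick sends it normalized axes from Center toward the X, Y and Z components, plus the world center and a fixed cube length.
; SetPlaneCenter, uncalled here, places the plane at the centroid of V1–V3, aligned to their triangle normal.
; CalcInvBasis is an empty stub.
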(event EventBeginPlay)

(event Collision|EventActorBeginOverlap
  (params (OtherActor :type Actor%20Object%20Reference)))

(event EventTick
  (params (DeltaSeconds :type Float%20%28single-precision%29))
  (Rendering|Material|SetVectorParameterValue (Variables|Default|GetDynMI) "x" (Math|Conversions|ToLinearColor(Vector) (Math|Vector|Normalize (- (Transformation|GetWorldLocation (Variables|组件|GetX)) (Transformation|GetWorldLocation (Variables|组件|GetCenter))))) :!class /Script/Engine.MaterialInstanceDynamic)
  (Rendering|Material|SetVectorParameterValue (Variables|Default|GetDynMI) "y" (Math|Conversions|ToLinearColor(Vector) (Math|Vector|Normalize (- (Transformation|GetWorldLocation (Variables|组件|GetY)) (Transformation|GetWorldLocation (Variables|组件|GetCenter))))) :!class /Script/Engine.MaterialInstanceDynamic)
  (Rendering|Material|SetVectorParameterValue (Variables|Default|GetDynMI) "z" (Math|Conversions|ToLinearColor(Vector) (Math|Vector|Normalize (- (Transformation|GetWorldLocation (Variables|组件|GetZ)) (Transformation|GetWorldLocation (Variables|组件|GetCenter))))) :!class /Script/Engine.MaterialInstanceDynamic)
  (Rendering|Material|SetVectorParameterValue (Variables|Default|GetDynMI) "cubecenter" (Math|Conversions|ToLinearColor(Vector) (Transformation|GetWorldLocation (Variables|组件|GetCenter))) :!class /Script/Engine.MaterialInstanceDynamic)
  (Rendering|Material|SetScalarParameterValue (Variables|Default|GetDynMI) "CubeLength" 5e+01 :!class /Script/Engine.MaterialInstanceDynamic))

(fn ConstructionScript
  (bind _returnvalue (Rendering|Material|CreateDynamicMaterialInstance (Variables|组件|GetPlane) 0 0 "None" :!class /Script/Engine.PrimitiveComponent))
  (bind _output_get (Variables|Default|SetDynMI _returnvalue))
  (Rendering|Material|SetMaterial (Variables|组件|GetPlane) 0 _output_get))

(fn CalcInvBasis)

(fn SetPlaneCenter
  (bind _v3 (Variables|组件|Getv3))
  (bind _relativelocation (Variables|/Script/Engine.SceneComponent|GetRelativeLocation _v3))
  (Transformation|SetRelativeLocationAndRotation (Variables|组件|GetPlane) (/ (+ (Variables|/Script/Engine.SceneComponent|GetRelativeLocation (Variables|组件|Getv1)) (Variables|/Script/Engine.SceneComponent|GetRelativeLocation (Variables|组件|Getv2)) (Variables|/Script/Engine.SceneComponent|GetRelativeLocation (Variables|组件|Getv3))) "3.000000,3.000000,3.000000") (Math|Rotator|MakeRotfromZ (Math|Vector|Normalize (Math|Vector|CrossProduct (- (Variables|/Script/Engine.SceneComponent|GetRelativeLocation (Variables|组件|Getv1)) _relativelocation) (- (Variables|/Script/Engine.SceneComponent|GetRelativeLocation (Variables|组件|Getv2)) _relativelocation)))) false false))