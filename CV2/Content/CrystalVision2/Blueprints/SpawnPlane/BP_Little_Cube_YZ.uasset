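; Spinning unit-cube actor that visualizes a crystallographic point, direction or plane, with optional physics.
; SetCube maps CubeStatus to a point marker, a scaled and rotated arrow, or a custom-mesh plane, also rebuilt at construction and BeginPlay.
; SetTriangle derives plane vertices from reciprocal-index axis intercepts, extruding along zero-index axes.
; SetNewLoc feeds coordinates back through SetCube, dividing by the smallest above-threshold component to get integer direction or plane indices.
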(event OnComponentHit(StaticMesh)
  (params (HitComponent :type Primitive%20Component%20Object%20Reference) (OtherActor :type Actor%20Object%20Reference) (OtherComp :type Primitive%20Component%20Object%20Reference) (NormalImpulse :type Vector :default "0, 0, 0") (Hit :type Hit%20Result%20Structure%20%28by%20ref%29))
  (Development|PrintString "Hello"))

(event EventBeginPlay
  (CallFunction|SetArrow)
  (CallFunction|SetPoint)
  (CallFunction|SetTriangle)
  (CallFunction|SetPhysics (Variables|Default|GetSimulate%20Physics)))

(event Collision|EventActorBeginOverlap
  (params (OtherActor :type Actor%20Object%20Reference)))

(event EventTick
  (params (DeltaSeconds :type Float%20%28single-precision%29))
  (Transformation|AddActorLocalRotation "0.000000,10.000000,0.000000" false false))

(fn ConstructionScript
  (CallFunction|SetArrow)
  (CallFunction|SetPoint)
  (CallFunction|SetTriangle)
  (CallFunction|SetPhysics (Variables|Default|GetSimulate%20Physics)))

(fn SetArrow
  (bind _arrow_visible (Variables|Arrow|GetArrow_Visible))
  (bind _arrow_x (Variables|Arrow|GetArrow_X))
  (bind _arrow_y (Variables|Arrow|GetArrow_Y))
  (bind _arrow_z (Variables|Arrow|GetArrow_Z))
  (bind _returnvalue (Math|Integer|Absolute(Integer) _arrow_x))
  (bind _returnvalue_2 (Math|Integer|Absolute(Integer) _arrow_y))
  (bind _returnvalue_3 (Math|Integer|Absolute(Integer) _arrow_z))
  (bind _returnvalue_4 (Math|Integer|Max(Integer) _returnvalue _returnvalue_2 _returnvalue_3))
  (bind _returnvalue_5 (> _returnvalue_4 0))
  (bind _returnvalue_6 (and _arrow_visible _returnvalue_5))
  (Rendering|SetVisibility (Variables|Default|GetTargetArrow) _returnvalue_6 false)
  (if _returnvalue_6
    (Utilities|FlowControl|Sequence
      (:then_0
        (bind _output_get (LocalVariables|SetVector (Math|Vector|MakeVector (Math|Conversions|ToFloat(Integer) _arrow_x) (Math|Conversions|ToFloat(Integer) _arrow_y) (Math|Conversions|ToFloat(Integer) _arrow_z))))
        (bind _output_get_2 (LocalVariables|SetVector (/ _output_get (Math|Conversions|ToFloat(Integer) _returnvalue_4))))
        (Transformation|SetRelativeScale3D (Variables|Default|GetTargetArrow) (Math|Vector|MakeVector (* (Math|Vector|VectorLength _output_get_2) 1.0 1.25) 1.0 1.0)))
      (:then_1
        (Transformation|SetRelativeLocationAndRotation (Variables|Default|GetTargetArrow) (Math|Vector|MakeVector (Math|Float|SelectFloat -5e+01 5e+01 (>= _arrow_x 0)) (Math|Float|SelectFloat -5e+01 5e+01 (>= _arrow_y 0)) (Math|Float|SelectFloat -5e+01 5e+01 (>= _arrow_z 0))) (Math|Conversions|RotationFromXVector (LocalVariables|GetVector)) false false)))))

(fn SetPoint
  (bind _point_visible (Variables|Point|GetPoint_Visible))
  (Rendering|SetVisibility (Variables|Default|GetTargetPoint) _point_visible false)
  (if _point_visible
    (Transformation|SetRelativeLocation (Variables|Default|GetTargetPoint) (- (* (Variables|Point|GetPointCoord) 1e+02) 5e+01) false false)))

(fn SetPlaneDontUse)

(fn SetTriangle
  (bind _notzeroxyz (LocalVariables|GetNotZeroXYZ))
  (bind _vertice (LocalVariables|GetVertice))
  (bind _plane_x (Variables|Plane|GetPlane_X))
  (bind _plane_y (Variables|Plane|GetPlane_Y))
  (bind _plane_z (Variables|Plane|GetPlane_Z))
  (bind _notzeroxyz_2 (LocalVariables|GetNotZeroXYZ))
  (bind _vertice_2 (LocalVariables|GetVertice))
  (bind _vertice_3 (LocalVariables|GetVertice))
  (bind _vertice_4 (LocalVariables|GetVertice))
  (bind _vertice_5 (LocalVariables|GetVertice))
  (bind _returnvalue (!= _plane_z 0))
  (bind _returnvalue_2 (!= _plane_x 0))
  (bind _returnvalue_3 (!= _plane_y 0))
  (Utilities|Array|SetArrayElem _notzeroxyz 0 _returnvalue_2)
  (Utilities|Array|SetArrayElem _notzeroxyz 1 _returnvalue_3)
  (Utilities|Array|SetArrayElem _notzeroxyz 2 _returnvalue)
  (bind _output_get (LocalVariables|SetCntNoneZero (+ (Math|Conversions|ToInteger(Boolean) _returnvalue) (Math|Conversions|ToInteger(Boolean) _returnvalue_3) (Math|Conversions|ToInteger(Boolean) _returnvalue_2))))
  (Rendering|SetVisibility (Variables|Default|GetCustomMesh) (and (Variables|Plane|GetPlane_Visible) (> _output_get 0)) false)
  (if (and (Variables|Plane|GetPlane_Visible) (> _output_get 0))
    (Utilities|FlowControl|Sequence
      (:then_0
        (bind _output_get_2 (LocalVariables|SetVertexOffset (Math|Vector|MakeVector (Math|Float|SelectFloat 0.0 1e+02 (>= _plane_x 0)) (Math|Float|SelectFloat 0.0 1e+02 (>= _plane_y 0)) (Math|Float|SelectFloat 0.0 1e+02 (>= _plane_z 0))))))
      (:then_1
        (if (Utilities|Array|Get(acopy) _notzeroxyz_2)
          (bind _output_get_3 (Variables|Plane|SetVertexX (Math|Vector|MakeVector (/ 1e+02 (Math|Conversions|ToFloat(Integer) _plane_x)) 0.0 0.0)))
          (bind _output_get_4 (Variables|Plane|SetVertexX (+ _output_get_3 _output_get_2)))
          (Utilities|Array|Add _vertice_4 _output_get_4)))
      (:then_2
        (if (Utilities|Array|Get(acopy) _notzeroxyz_2 1)
          (bind _output_get_5 (Variables|Plane|SetVertexY (Math|Vector|MakeVector 0.0 (/ 1e+02 (Math|Conversions|ToFloat(Integer) _plane_y)) 0.0)))
          (bind _output_get_6 (Variables|Plane|SetVertexY (+ _output_get_5 _output_get_2)))
          (Utilities|Array|Add _vertice_4 _output_get_6)))
      (:then_3
        (if (Utilities|Array|Get(acopy) _notzeroxyz_2 2)
          (bind _output_get_7 (Variables|Plane|SetVertexZ (Math|Vector|MakeVector 0.0 0.0 (/ 1e+02 (Math|Conversions|ToFloat(Integer) _plane_z)))))
          (bind _output_get_8 (Variables|Plane|SetVertexZ (+ _output_get_7 _output_get_2)))
          (Utilities|Array|Add _vertice_4 _output_get_8)))
      (:then_4
        (switch int (LocalVariables|GetCntNoneZero)
          (:1
            (Utilities|Array|SetArrayElem _vertice_5 0 (Math|Vector|ClampVectorSize (Utilities|Array|Get(acopy) _vertice_5) 0.5 99.5))
            (bind (_array_element _array_index) (Utilities|Array|ForEachLoopwithBreak (LocalVariables|GetNotZeroXYZ) :!label _label)
              (:LoopBody
                (if (< _array_index 3)
                  (if (not _array_element)
                    (bind _output_get_9 (LocalVariables|SettempCnt (+ (LocalVariables|GettempCnt) 1)))
                    (bind (_array_element_2 _array_index_2) (Utilities|Array|ForEachLoopwithBreak (LocalVariables|GetVertice) :!label _label_2)
                      (:LoopBody
                        (if (< _array_index_2 _output_get_9)
                          (Utilities|Array|Add (LocalVariables|GetVertice) (+ _array_element_2 (Utilities|Select :Index _array_index :Option%200 "100.000000, 0, 0" :Option%201 "0.000000,100.000000, 0" :Option%202 "0,0.000000,100.000000")))
                          (else
                            (goto _label_2 Break))))))
                  (else
                    (goto _label Break))))
              (:Completed
                (Class|CustomMeshComponent|SetCustomMeshTriangles (Variables|Default|GetCustomMesh) (Utilities|Array|MakeArray (Utilities|Struct|MakeCustomMeshTriangle (Utilities|Array|Get(acopy) _vertice_2) (Utilities|Array|Get(acopy) _vertice_2 1) (Utilities|Array|Get(acopy) _vertice_2 2)) (Utilities|Struct|MakeCustomMeshTriangle (Utilities|Array|Get(acopy) _vertice_2 1) (Utilities|Array|Get(acopy) _vertice_2 2) (Utilities|Array|Get(acopy) _vertice_2 3)))))))
          (:2
            (bind (_array_element_3 _array_index_3) (Utilities|Array|ForEachLoopwithBreak (LocalVariables|GetVertice) :!label _label_3)
              (:LoopBody
                (if (< _array_index_3 2)
                  (Utilities|Array|Add (LocalVariables|GetVertice) (+ _array_element_3 (Utilities|Select :Index (Utilities|Array|FindItem (LocalVariables|GetNotZeroXYZ) false) :Option%200 "100.000000, 0, 0" :Option%201 "0.000000,100.000000, 0" :Option%202 "0,0.000000,100.000000")))
                  (else
                    (goto _label_3 Break))))
              (:Completed
                (Class|CustomMeshComponent|ClearCustomMeshTriangles (Variables|Default|GetCustomMesh))
                (Class|CustomMeshComponent|SetCustomMeshTriangles (Variables|Default|GetCustomMesh) (Utilities|Array|MakeArray (Utilities|Struct|MakeCustomMeshTriangle (Utilities|Array|Get(acopy) _vertice_3) (Utilities|Array|Get(acopy) _vertice_3 1) (Utilities|Array|Get(acopy) _vertice_3 2)) (Utilities|Struct|MakeCustomMeshTriangle (Utilities|Array|Get(acopy) _vertice_3 1) (Utilities|Array|Get(acopy) _vertice_3 2) (Utilities|Array|Get(acopy) _vertice_3 3)))))))
          (:3
            (Class|CustomMeshComponent|SetCustomMeshTriangles (Variables|Default|GetCustomMesh) (Utilities|Array|MakeArray (Utilities|Struct|MakeCustomMeshTriangle (Utilities|Array|Get(acopy) _vertice) (Utilities|Array|Get(acopy) _vertice 1) (Utilities|Array|Get(acopy) _vertice 2))))))))))

(fn SetPhysics
  (params (IsPhysics :type Boolean))
  (Physics|SetSimulatePhysics (Variables|Default|GetStaticMesh) IsPhysics))

(fn SetCube
  (params (CubeStatus :type Structure%20Cube%20Status%20Structure) (Editable :type Boolean) (SimulatePhysics :type Boolean))
  (Variables|Default|SetEditable Editable)
  (bind _output_get (Variables|Default|SetSimulate%20Physics SimulatePhysics))
  (CallFunction|SetPhysics _output_get)
  (bind _output_get_2 (Variables|Default|SetCube%20Status CubeStatus))
  (switch Utilities|FlowControl|Switch|Switchonenum_CubeType (.CubeType (Utilities|Struct|BreakStructure_CubeStatus _output_get_2))
    (:NewEnumerator0
      (Variables|Point|SetPoint_Visible true)
      (Variables|Point|SetPointCoord (.ValuesXYZ (Utilities|Struct|BreakStructure_CubeStatus _output_get_2)))
      (CallFunction|SetPoint))
    (:NewEnumerator1
      (Variables|Arrow|SetArrow_Visible true)
      (Variables|Arrow|SetArrow_X (Math|Conversions|ToInteger(Byte) (Class|KismetMathLibrary|Round64 (.X (Math|Vector|BreakVector (.ValuesXYZ (Utilities|Struct|BreakStructure_CubeStatus _output_get_2)))))))
      (Variables|Arrow|SetArrow_Y (Math|Conversions|ToInteger(Byte) (Class|KismetMathLibrary|Round64 (.Y (Math|Vector|BreakVector (.ValuesXYZ (Utilities|Struct|BreakStructure_CubeStatus _output_get_2)))))))
      (Variables|Arrow|SetArrow_Z (Math|Conversions|ToInteger(Byte) (Class|KismetMathLibrary|Round64 (.Z (Math|Vector|BreakVector (.ValuesXYZ (Utilities|Struct|BreakStructure_CubeStatus _output_get_2)))))))
      (CallFunction|SetArrow))
    (:NewEnumerator2
      (Variables|Plane|SetPlane_Visible true)
      (Variables|Plane|SetPlane_X (Math|Conversions|ToInteger(Byte) (Class|KismetMathLibrary|Round64 (.X (Math|Vector|BreakVector (.ValuesXYZ (Utilities|Struct|BreakStructure_CubeStatus _output_get_2)))))))
      (Variables|Plane|SetPlane_Y (Math|Conversions|ToInteger(Byte) (Class|KismetMathLibrary|Round64 (.Y (Math|Vector|BreakVector (.ValuesXYZ (Utilities|Struct|BreakStructure_CubeStatus _output_get_2)))))))
      (Variables|Plane|SetPlane_Z (Math|Conversions|ToInteger(Byte) (Class|KismetMathLibrary|Round64 (.Z (Math|Vector|BreakVector (.ValuesXYZ (Utilities|Struct|BreakStructure_CubeStatus _output_get_2)))))))
      (CallFunction|SetTriangle))))

(fn SetInitStatus)

(fn SetNewLoc
  (params (Coord :type Vector))
  (bind (_x _y _z) (Math|Vector|BreakVector Coord))
  (bind _temparray (LocalVariables|GetTempArray))
  (bind _temparray_2 (LocalVariables|GetTempArray))
  (Utilities|Array|SetArrayElem _temparray_2 0 _x true)
  (Utilities|Array|SetArrayElem _temparray_2 1 _y true)
  (Utilities|Array|SetArrayElem _temparray_2 2 _z true)
  (for (_array_element _array_index) _temparray_2
    (if (> _array_element (LocalVariables|GetThreshold))
      (if (> (LocalVariables|Getmin) _array_element)
        (LocalVariables|Setmin _array_element))
      (else
        (Utilities|Array|SetArrayElem (LocalVariables|GetTempArray) _array_index 0.0))))
  (bind _output_get (Variables|Default|SetCube%20Status (Utilities|Struct|MakeStructure_CubeStatus (.CubeType (Utilities|Struct|BreakStructure_CubeStatus (Variables|Default|GetCube%20Status))) (Utilities|Select :Index (.CubeType (Utilities|Struct|BreakStructure_CubeStatus (Variables|Default|GetCube%20Status))) :NewEnumerator0 Coord :NewEnumerator1 (Math|Vector|MakeVector (Math|Conversions|ToFloat(Integer) (Math|Float|Round (/ (Utilities|Array|Get(acopy) _temparray) (LocalVariables|Getmin)))) (Math|Conversions|ToFloat(Integer) (Math|Float|Round (/ (Utilities|Array|Get(acopy) _temparray 1) (LocalVariables|Getmin)))) (Math|Conversions|ToFloat(Integer) (Math|Float|Round (/ (Utilities|Array|Get(acopy) _temparray 2) (LocalVariables|Getmin))))) :NewEnumerator2 (Math|Vector|MakeVector (Math|Conversions|ToFloat(Integer) (Math|Float|Round (/ (Utilities|Array|Get(acopy) _temparray) (LocalVariables|Getmin)))) (Math|Conversions|ToFloat(Integer) (Math|Float|Round (/ (Utilities|Array|Get(acopy) _temparray 1) (LocalVariables|Getmin)))) (Math|Conversions|ToFloat(Integer) (Math|Float|Round (/ (Utilities|Array|Get(acopy) _temparray 2) (LocalVariables|Getmin)))))))))
  (CallFunction|SetCube _output_get (Variables|Default|GetEditable) (Variables|Default|GetSimulate%20Physics)))

(fn GetCoord
  (return (.ValuesXYZ (Utilities|Struct|BreakStructure_CubeStatus (Variables|Default|GetCube%20Status)))))