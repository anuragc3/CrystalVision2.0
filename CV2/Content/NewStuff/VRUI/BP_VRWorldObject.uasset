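; World-space VR UI actor that holds the game's menu widget components, such as main menu, pause, credits, level info and game over.
; BeginPlay selects the VR controls widget, lowers every panel out of the way and shows the main menu on Outdoor1.
; Show switches panels by enum, toggling visibility and shifting them vertically, with CurrentWidget and HoldUI tracking the active one.
; CheckAnyVisible reports whether any panel is visible.
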(event EventBeginPlay
  (Variables|Default|SetControlWidgetType (Variables|Default|GetControls_Widget_VR))
  (CallFunction|MoveWidget)
  (bind _returnvalue (Game|GetCurrentLevelName true))
  (CallFunction|Show "NewEnumerator1" (Utilities|Enum|Equal(Enum) _returnvalue "Outdoor1")))

(event Collision|EventActorBeginOverlap
  (params (OtherActor :type Actor%20Object%20Reference)))

(event EventTick
  (params (DeltaSeconds :type Float%20%28single-precision%29)))

(fn ConstructionScript)

(fn Show
  (params (UI_widget :type Enum_UI%20Enum :default "NewEnumerator0") (On%20/%20Off :type Boolean))
  (bind _mainmenumiddle_widget (Variables|Default|GetMainMenuMiddle_Widget))
  (bind _levelinfo2_widget (Variables|Default|GetLevelInfo2_Widget))
  (bind _info_widget (Variables|Default|GetInfo_Widget))
  (bind _gameovermenu_widget (Variables|Default|GetGameOverMenu_Widget))
  (bind _levelfinishes_widget (Variables|Default|GetLevelFinishes_Widget))
  (bind _controlwidgettype (Variables|Default|GetControlWidgetType))
  (bind _pause_widget (Variables|Default|GetPause_Widget))
  (bind _mainmenu_widget (Variables|Default|GetMainMenu_Widget))
  (bind _credits_widget (Variables|Default|GetCredits_Widget))
  (bind _end_widget (Variables|Default|GetEnd_Widget))
  (bind _levelinfo1_widget (Variables|Default|GetLevelInfo1_Widget))
  (bind _levelinfo3_widget (Variables|Default|GetLevelInfo3_Widget))
  (bind _returnvalue (Utilities|Select :Index UI_widget :NewEnumerator0 _pause_widget :NewEnumerator1 _mainmenu_widget :NewEnumerator2 _credits_widget :NewEnumerator3 _controlwidgettype :NewEnumerator4 _end_widget :NewEnumerator5 _levelinfo1_widget :NewEnumerator6 _levelinfo2_widget :NewEnumerator7 _levelinfo3_widget :NewEnumerator8 _info_widget :NewEnumerator9 _mainmenumiddle_widget :NewEnumerator10 _gameovermenu_widget :NewEnumerator11 _levelfinishes_widget))
  (if (Variables|Default|GetHoldUI)
    (bind _as控件组件 (Utilities|Casting|CastToWidgetComponent (Variables|Default|GetCurrentWidget)))
    (Transformation|AddRelativeLocation _as控件组件 "0, 0,-2000.000000" false false)
    (Rendering|SetVisibility _as控件组件 false false))
  (if On%20/%20Off
    (Transformation|AddRelativeLocation _returnvalue "0.000000, 0,2000.000000" false false)
    (Rendering|SetVisibility _returnvalue true false)
    (Variables|Default|SetCurrentWidget _returnvalue)
    (Variables|Default|SetHoldUI true)
    (else
      (Variables|Default|SetHoldUI false))))

(fn CheckAnyVisible
  (for _array_element (Utilities|Array|MakeArray (Variables|Default|GetCredits_Widget) (Variables|Default|GetLevelFinishes_Widget) (Variables|Default|GetMainMenuMiddle_Widget) (Variables|Default|GetMainMenu_Widget) (Variables|Default|GetEnd_Widget) (Variables|Default|GetInfo_Widget) (Variables|Default|GetPause_Widget) (Variables|Default|GetControlWidgetType) (Variables|Default|GetLevelInfo1_Widget) (Variables|Default|GetLevelInfo2_Widget) (Variables|Default|GetLevelInfo3_Widget) (Variables|Default|GetGameOverMenu_Widget))
    (if (Rendering|IsVisible _array_element)
      (return true)))
  (return false))

(fn MoveWidget
  (for _array_element (Utilities|Array|MakeArray (Variables|Default|GetCredits_Widget) (Variables|Default|GetLevelFinishes_Widget) (Variables|Default|GetMainMenuMiddle_Widget) (Variables|Default|GetMainMenu_Widget) (Variables|Default|GetEnd_Widget) (Variables|Default|GetInfo_Widget) (Variables|Default|GetPause_Widget) (Variables|Default|GetControlWidgetType) (Variables|Default|GetLevelInfo1_Widget) (Variables|Default|GetLevelInfo2_Widget) (Variables|Default|GetLevelInfo3_Widget) (Variables|Default|GetGameOverMenu_Widget))
    (Transformation|AddRelativeLocation _array_element "0, 0,-2000.000000" false false)))