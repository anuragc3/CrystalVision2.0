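; A demo portal actor that sends the darts VR pawn to another level when that pawn enters its box.
; The overlap casts to MotionControllerPawn_Darts and opens the hard-referenced level Lab2Level4.
; The construction script sets the label from DisplayText and applies a cull distance to it.
; An older in-level teleport, with level number, unlock record, control panel and quiz restart logic, remains disconnected and never runs.
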(event OnComponentBeginOverlap(Box)
  (params (OverlappedComponent :type Primitive%20Component%20Object%20Reference) (OtherActor :type Actor%20Object%20Reference) (OtherComp :type Primitive%20Component%20Object%20Reference) (OtherBodyIndex :type Integer) (bFromSweep :type Boolean) (SweepResult :type Hit%20Result%20Structure%20%28by%20ref%29))
  (bind _asmotion_controller_pawn_darts (Utilities|Casting|CastToMotionControllerPawn_Darts OtherActor))
  (Game|OpenLevel(byObjectReference) "/Game/CrystalVision2/Levels/Lab2Level4.Lab2Level4"))

(event EventBeginPlay)

(event Collision|EventActorBeginOverlap
  (params (OtherActor :type Actor%20Object%20Reference)))

(event EventTick
  (params (DeltaSeconds :type Float%20%28single-precision%29)))

(fn ConstructionScript
  (Rendering|Components|TextRender|SetText (Variables|Default|GetTextRender) (Variables|Default|GetDisplayText))
  (Class|PrimitiveComponent|SetCullDistance (Variables|Default|GetTextRender) 3.5e+03))