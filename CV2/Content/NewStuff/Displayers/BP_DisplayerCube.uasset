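; Display stand for an interactive BP_Cube1 that demonstrates points, directions or planes with HKL indices.
; BeginPlay spawns and attaches the cube from CubeInfo, adding three BP_PlaneHKLSelector actors for cube type 2, with UpdateHKL passing values to the cube's plane.
; Tick shows point or direction coordinates as text.
; Motion controller or bullet overlap with the Box resets the cube's setup and transform and clears its points.
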(event OnComponentBeginOverlap(Box)
  (params (OverlappedComponent :type Primitive%20Component%20Object%20Reference) (OtherActor :type Actor%20Object%20Reference) (OtherComp :type Primitive%20Component%20Object%20Reference) (OtherBodyIndex :type Integer) (bFromSweep :type Boolean) (SweepResult :type Hit%20Result%20Structure%20%28by%20ref%29))
  (Utilities|Casting|CastToBP_MotionController_Darts OtherActor
    (:then
      _)
    (:CastFailed
      (Utilities|Casting|CastToBP_Bullet OtherActor)))
  (CallFunction|Reset))

(event EventBeginPlay
  (bind _returnvalue (Game|SpawnActorfromClass "/Game/NewStuff/Cubes/BP_Cube1.BP_Cube1_C" (Math|Transform|MakeTransform (Variables|Default|GetOffset) "0, 0, 0" "1.000000,1.000000,1.000000") "Undefined" "OverrideRootScale" 0 0))
  (Transformation|AttachActorToActor _returnvalue self "None" "KeepRelative" "KeepRelative" "KeepRelative" true)
  (Utilities|FlowControl|Sequence
    (:then_0
      (bind _output_get (Variables|Default|SetCube _returnvalue))
      (Variables|Default|SetGotCube true)
      (Default|SetCube (Variables|Default|GetCube) (Variables|Default|GetCubeInfo) (Variables|Default|GetCubeEditable) false)
      (Variables|Default|SetOldTransform (Transformation|GetActorTransform (Variables|Default|GetCube)))
      (if (== (.CubeType (Utilities|Struct|BreakStructure_CubeStatus (Variables|Default|GetCubeInfo))) 2)
        (Utilities|FlowControl|Sequence
          (:then_0
            (bind _returnvalue_2 (Game|SpawnActorfromClass "/Game/CrystalVision2/Blueprints/Common/BP_PlaneHKLSelector.BP_PlaneHKLSelector_C" (Math|Transform|MakeTransform "30.000000,100.000000,370.000000" "0, 0, 0" "1.000000,1.000000,1.000000") "Undefined" "MultiplyWithRoot" 0 0))
            (bind _output_get_2 (Variables|Default|SetHKLH _returnvalue_2))
            (Variables|/Game/CrystalVision2/Blueprints/Common/BP_PlaneHKLSelector.BP_PlaneHKLSelector_C|SetDisplayer _output_get_2 self)
            (Variables|/Game/CrystalVision2/Blueprints/Common/BP_PlaneHKLSelector.BP_PlaneHKLSelector_C|SetHKLidx _output_get_2 0)
            (Transformation|AttachActorToActor _output_get_2 self "None" "KeepRelative" "KeepRelative" "KeepRelative" true))
          (:then_1
            (bind _returnvalue_3 (Game|SpawnActorfromClass "/Game/CrystalVision2/Blueprints/Common/BP_PlaneHKLSelector.BP_PlaneHKLSelector_C" (Math|Transform|MakeTransform "30.000000,0.000000,370.000000" "0, 0, 0" "1.000000,1.000000,1.000000") "Undefined" "MultiplyWithRoot" 0 0))
            (bind _output_get_3 (Variables|Default|SetHKLK _returnvalue_3))
            (Variables|/Game/CrystalVision2/Blueprints/Common/BP_PlaneHKLSelector.BP_PlaneHKLSelector_C|SetDisplayer _output_get_3 self)
            (Variables|/Game/CrystalVision2/Blueprints/Common/BP_PlaneHKLSelector.BP_PlaneHKLSelector_C|SetHKLidx _output_get_3 1)
            (Transformation|AttachActorToActor _output_get_3 self "None" "KeepRelative" "KeepRelative" "KeepRelative" true))
          (:then_2
            (bind _returnvalue_4 (Game|SpawnActorfromClass "/Game/CrystalVision2/Blueprints/Common/BP_PlaneHKLSelector.BP_PlaneHKLSelector_C" (Math|Transform|MakeTransform "30.000000,-100.000000,370.000000" "0, 0, 0" "1.000000,1.000000,1.000000") "Undefined" "MultiplyWithRoot" 0 0))
            (bind _output_get_4 (Variables|Default|SetHKLL _returnvalue_4))
            (Variables|/Game/CrystalVision2/Blueprints/Common/BP_PlaneHKLSelector.BP_PlaneHKLSelector_C|SetDisplayer _output_get_4 self)
            (Variables|/Game/CrystalVision2/Blueprints/Common/BP_PlaneHKLSelector.BP_PlaneHKLSelector_C|SetHKLidx _output_get_4 2)
            (Transformation|AttachActorToActor _output_get_4 self "None" "KeepRelative" "KeepRelative" "KeepRelative" true)))))
    (:then_1
      (Default|ChangeMobility _output_get "Stationary"))))

(event Collision|EventActorBeginOverlap
  (params (OtherActor :type Actor%20Object%20Reference)))

(event EventTick
  (params (DeltaSeconds :type Float%20%28single-precision%29))
  (if (Variables|Default|GetGotCube)
    (CallFunction|PrintInfo)))

(fn ConstructionScript
  (Class|PrimitiveComponent|SetCullDistance (Variables|Default|GetTextRender) 3.5e+03)
  (Class|PrimitiveComponent|SetCullDistance (Variables|Default|GetTextRender1) 3.5e+03)
  (Class|PrimitiveComponent|SetCullDistance (Variables|Default|GetTextRender2) 3.5e+03)
  (Class|PrimitiveComponent|SetCullDistance (Variables|Default|GetTextRender3) 3.5e+03)
  (Class|PrimitiveComponent|SetCullDistance (Variables|Default|GetTextRender4) 3.5e+03)
  (Class|PrimitiveComponent|SetCullDistance (Variables|Default|GetTextRender5) 3.5e+03)
  (Class|PrimitiveComponent|SetCullDistance (Variables|Default|GetTextRender6) 3.5e+03)
  (Class|PrimitiveComponent|SetCullDistance (Variables|Default|GetArrowText) 3.5e+03)
  (Class|PrimitiveComponent|SetCullDistance (Variables|Default|GetPlaneText) 3.5e+03)
  (Class|PrimitiveComponent|SetCullDistance (Variables|Default|GetPointText) 3.5e+03))

(fn PrintInfo
  (bind _ret (Default|GetCoord (Variables|Default|GetCube)))
  (Rendering|Components|TextRender|SetText (Variables|Default|GetPointText) (Utilities|Select :Index (.CubeType (Utilities|Struct|BreakStructure_CubeStatus (Variables|Default|GetCubeInfo))) :NewEnumerator0 (Utilities|Text|ToText(String) _ret) :NewEnumerator1 (Utilities|Text|FormatText (Utilities|Text|MakeLiteralText "{0}  {1}  {2}") (Math|Float|Round (.X (Math|Vector|BreakVector _ret))) (Math|Float|Round (.Y (Math|Vector|BreakVector _ret))) (Math|Float|Round (.Z (Math|Vector|BreakVector _ret)))) :NewEnumerator2 "")))

(fn Reset
  (bind _cube (Variables|Default|GetCube))
  (Default|CallHoldertoDrop _cube)
  (Default|ChangeMobility _cube "Movable")
  (Default|SetCube _cube (Variables|Default|GetCubeInfo) (Variables|Default|GetCubeEditable) false)
  (Transformation|SetActorTransform _cube (Variables|Default|GetOldTransform))
  (Default|ChangeMobility _cube "Stationary")
  (Default|DestroyAllPoints (Variables|Default|GetCube)))

(fn UpdateHKL
  (params (idx :type Integer) (value :type Integer))
  (Utilities|Array|SetArrayElem (Variables|Default|GetHKL) idx value)
  (Default|SetPlaneCenter (Variables|Default|GetCube) (Variables|Default|GetHKL)))

(fn HKLtoXYZ
  (bind _hkl (Variables|Default|GetHKL))
  (bind _output (Utilities|Array|Get(acopy) _hkl))
  (if (== 0 _output)
    (LocalVariables|Setx 0)
    (else
      (LocalVariables|Setx (/ 1 _output))))
  (if (> 0 _output)
    (LocalVariables|Setxoff 1)
    (else
      (LocalVariables|Setxoff 0))))